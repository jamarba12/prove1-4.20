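; BP_GameRules holds the game rules: enemy generation timing, score and player respawn.
; On BeginPlay it starts a looping timer that calls Enemies Verification on the first EnemyGenerator found, at an interval derived from EnemiesNumberBySecond.
; Respawnplayer destroys all enemies and their weapons, resets Score, then spawns and possesses a new BP_Player at TransPlacePlayer.
; IncreaseScore adds one to Score.
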(event `self.ReceiveBeginPlay`
  ;[1 1 1] Generate new enemies
  (bind _outactors (`GameplayStatics.GetAllActorsOfClass` "/Game/Blueprints/Enemy/EnemyGenerator.EnemyGenerator_C"))
  (bind _output_get (set `self.Generator Volumen` (`|GetArrayItem` _outactors)))
  (`KismetSystemLibrary.K2_SetTimer` _output_get "Enemies Verification" (/ 1.0 (`self.Enemies Number by second`)) true))

(event `Respawn player`
  ;[1 1 1] Respawn player
  (bind _outactors (`GameplayStatics.GetAllActorsOfClass` "/Game/Blueprints/Enemy/Pawns/BP_EnemyBase.BP_EnemyBase_C"))
  (for _array_element _outactors
    (`self.K2_DestroyActor` _array_element)
    (`self.K2_DestroyActor` (`/Game/Blueprints/Enemy/Pawns/BP_EnemyBase.Weapon` _array_element)))
  (set `self.Score` 0.0)
  (bind _returnvalue (`|SpawnActorFromClass` "/Game/Blueprints/BP_Player.BP_Player_C" (`self.Trans_place_player`) "Undefined" "OverrideRootScale" null null))
  (`Controller.Possess` (`GameplayStatics.GetPlayerController` 0) _returnvalue))

(fn `Increase Score`
  (`/Engine/EditorBlueprintResources/StandardMacros.IncrementFloat` (`self.Score`)))

(fn `UserConstructionScript`)