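; BP_EnemyBase is the base enemy pawn with health that can be damaged and killed.
; On BeginPlay it spawns a BP_Weapon and attaches it to the mesh's right-hand socket.
; MakeDamage subtracts health and updates the Living flag; on death it increases the score through BP_GameRules, then destroys both the weapon and itself.
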(event `self.ReceiveBeginPlay`
  (bind _returnvalue (`|SpawnActorFromClass` "/Game/Blueprints/Enemy/BP_Weapon.BP_Weapon_C" (`SceneComponent.K2_GetComponentToWorld` (`self.Mesh`)) "AlwaysSpawn" "OverrideRootScale" null null))
  (bind _output_get (set `self.Weapon` _returnvalue))
  (`self.K2_AttachToComponent` _output_get (`self.Mesh`) "hand_rSocket" "SnapToTarget" "SnapToTarget" "SnapToTarget" true))

(event `/Game/Blueprints/Interface.Make Damage`
  (params (`Making Damage` :type "Float (single-precision)"))
  (`self.Calculate Health` `Making Damage`)
  (if (not (`self.Living`))
    (bind _asbp_game_rules (cast `/Game/Blueprints/BP_GameRules` (`GameplayStatics.GetGameMode`)))
    (`/Game/Blueprints/BP_GameRules.Increase Score` _asbp_game_rules)
    (`self.K2_DestroyActor` (`self.Weapon`))
    (`self.K2_DestroyActor` self)))

(fn `Calculate Death`
  (if (<= (`self.Health`) 0.0)
    (set `self.Living` false)
    (else
      (set `self.Living` true))))

(fn `Calculate Health`
  (params (Damage :type "Float (double-precision)"))
  (locals (NewLocalVar_0 :type "Float (double-precision)" :default 0.0))
  (set `self.Health` (- (`self.Health`) Damage))
  (`self.Calculate Death`))

(fn `UserConstructionScript`)