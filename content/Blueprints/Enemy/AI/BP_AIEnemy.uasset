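; AI controller for enemy pawns that runs the enemy behavior tree and drives their weapon fire from perception.
; On possessing a BP_EnemyBase, it starts BT_enemy.
; When perception of the player updates, it writes the ICanSee? blackboard key and squeezes the pawn's weapon trigger when sensed or releases it when lost.
; A Deprecated graph keeps an unused timer and move-to player chase.
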(event `self.ReceiveBeginPlay`)

(event `LookforPlayer`)

(event `self.OnPossess`
  (params (PossessedPawn :type "Pawn Object Reference"))
  (cast `/Game/Blueprints/Enemy/Pawns/BP_EnemyBase` PossessedPawn)
  (`self.RunBehaviorTree` "/Game/Blueprints/Enemy/AI/BT_enemy.BT_enemy"))

(event `self.AIPerception.OnTargetPerceptionUpdated`
  (params (Actor :type "Actor Object Reference") (Stimulus :type "AIStimulus Structure"))
  (bind (_age _expirationage _strength _stimuluslocation _receiverlocation _tag _bsuccessfullysensed) (break `AIStimulus` Stimulus))
  (bind _returnvalue (`self.K2_GetPawn`))
  (cast `/Game/Blueprints/BP_Player` Actor)
  (`BlackboardComponent.SetValueAsBool` (`AIBlueprintHelperLibrary.GetBlackboard` null) "ICanSee?" _bsuccessfullysensed)
  (if _bsuccessfullysensed
    (bind _asbp_enemy_base (cast `/Game/Blueprints/Enemy/Pawns/BP_EnemyBase` _returnvalue))
    (`/Game/Blueprints/Enemy/BP_Weapon.Squeeze Trigger` (`/Game/Blueprints/Enemy/Pawns/BP_EnemyBase.Weapon` _asbp_enemy_base))
    (else
      (bind _asbp_enemy_base_2 (cast `/Game/Blueprints/Enemy/Pawns/BP_EnemyBase` _returnvalue))
      (`/Game/Blueprints/Enemy/BP_Weapon.Release Trigger` (`/Game/Blueprints/Enemy/Pawns/BP_EnemyBase.Weapon` _asbp_enemy_base_2)))))

(fn `UserConstructionScript`)