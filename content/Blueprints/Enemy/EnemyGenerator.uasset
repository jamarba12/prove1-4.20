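; Enemy generator that tops up the enemy population by spawning AI pawns inside its volume.
; Its EnemiesVerification event counts actors tagged "Bad ones" and, while the count is at or below a small fixed cap, spawns one random class from EnemiesList.
; Each spawn runs the BT_enemy behavior tree and lands at a random point within the GeneratorVolumen box.
; Nothing in this Blueprint calls that event.
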(event `Enemies Verification`
  (bind _enemies_list (`self.Enemies list`))
  (bind _generator_volumen (`self.Generator Volumen`))
  (bind _outactors (`GameplayStatics.GetAllActorsWithTag` "Bad ones"))
  (bind _output_get (set `self.Playing Enemy Number` (`KismetArrayLibrary.Array_Length` _outactors)))
  (if (<= _output_get 5)
    (`AIBlueprintHelperLibrary.SpawnAIFromClass` (`|GetArrayItem` _enemies_list (`KismetMathLibrary.RandomIntegerInRange` 0 (`KismetArrayLibrary.Array_LastIndex` _enemies_list))) "/Game/Blueprints/Enemy/AI/BT_enemy.BT_enemy" (`KismetMathLibrary.RandomPointInBoundingBox` (`SceneComponent.K2_GetComponentLocation` _generator_volumen) (`BoxComponent.BoxExtent` _generator_volumen)))))

(fn `UserConstructionScript`)